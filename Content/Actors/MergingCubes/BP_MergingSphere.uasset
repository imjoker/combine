(event `self.ReceiveBeginPlay`
  (bind _returnvalue (`KismetMaterialLibrary.CreateDynamicMaterialInstance` (`PrimitiveComponent.GetMaterial` (`self.StaticMeshComponent`) 0)))
  (set `self.NewVar_0` _returnvalue)
  (`PrimitiveComponent.SetMaterial` (`self.StaticMeshComponent`) 0 _returnvalue))

(event `/Game/Actors/MergingCubes/EventCubeOnFire.CubeOnFire`
  ;[1 1 1] SetOnFireUponTrigger
  (if (not (`self.IsEmitterActive`))
    (bind _returnvalue (`GameplayStatics.SpawnEmitterAttached` "/Game/StarterContent/Particles/P_Fire.P_Fire" (`self.StaticMeshComponent`) "None" (0.0 0.0 0.0) (struct) (2.0 1.5 2.0) "SnapToTargetIncludingScale"))
    (set `self.IsEmitterActive` true)
    (set `self.FireEmitter` _returnvalue)))

(event `self.ReceiveActorBeginOverlap`
  (params (OtherActor :type "Actor Object Reference"))
  ;[1 1 1] DissolveFireIntoSmokeAndChangeColorToRed
  (if (`self.ActorHasTag` OtherActor "Water")
    (if (`self.IsEmitterActive`)
      (bind _returnvalue (`GameplayStatics.SpawnEmitterAtLocation` "/Game/StarterContent/Particles/P_Steam_Lit.P_Steam_Lit" (`self.K2_GetActorLocation`) (struct) (2.0 2.0 2.0)))
      (set `self.IsEmitterActive` false)
      (`ActorComponent.Deactivate` (`self.FireEmitter`))
      (if (`self.ActorHasTag` OtherActor "Red")
        (`PrimitiveComponent.SetMaterial` (`self.StaticMeshComponent`) 0 (`self.Red`))
        (`KismetSystemLibrary.Delay` 5.0)
        (`ActorComponent.Deactivate` _returnvalue))
      (else
        (`PrimitiveComponent.SetMaterial` (`self.StaticMeshComponent`) 0 (`self.Red`))))))

(fn `UserConstructionScript`)