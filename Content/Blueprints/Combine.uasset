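; Combine is an actor component that merges its owner with another component's owner by spawning a combined actor.
; Merge spawns the Output class at the other owner's location, with zero rotation and both owners' scales summed, then applies a purple merge material.
; Delete separately destroys the owning actor, as Merge leaves both source actors in place.
; A midpoint spawn-location calculation is present but unused.
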(fn `Delete`
  (`Actor.K2_DestroyActor` (`self.GetOwner`)))

(fn `Merge`
  (params (Other :type "/Game/Blueprints/Combine Object Reference"))
  (bind _returnvalue (`self.GetOwner` Other))
  (bind _returnvalue_2 (`|SpawnActorFromClass` (`self.Output`) (`KismetMathLibrary.MakeTransform` (`Actor.K2_GetActorLocation` _returnvalue) (struct) (+ (`Actor.GetActorScale3D` _returnvalue) (`Actor.GetActorScale3D` (`self.GetOwner`)))) "Undefined" "OverrideRootScale" null null))
  (`PrimitiveComponent.SetMaterial` (`Actor.GetComponentByClass` _returnvalue_2 "/Script/Engine.PrimitiveComponent") 0 "/Game/Actors/MergingCubes/MergingColorPurple.MergingColorPurple"))