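; BP_Square_Tier2 is a square actor, apparently a second-tier piece for a combine mechanic, with a cube mesh and box collision.
; At BeginPlay it applies the Simulate flag to the box's physics and picks a random ID.
; Its level-based material, geometrically compounded sizing via Pure, and timeline growth to the next level are all disconnected.
; Tick, hit, overlap, animation and construction entry points are empty.
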(event `self.ReceiveTick`
  (params (DeltaSeconds :type "Float (single-precision)")))

(event `ANIMATION`
  ;[1 1 1] animation
)

(event `self.ReceiveBeginPlay`
  (`PrimitiveComponent.SetSimulatePhysics` (`self.Box`) (`self.Simulate`))
  (set `self.ID` (`KismetMathLibrary.RandomIntegerInRange` 0 999)))

(event `self.Box.OnComponentHit`
  (params (HitComponent :type "PrimitiveComponent Object Reference") (OtherActor :type "Actor Object Reference") (OtherComp :type "PrimitiveComponent Object Reference") (NormalImpulse :type "Vector Structure") (Hit :type "HitResult Structure (by ref)")))

(fn `pure`
  (params (A :type "Vector Structure") (B :type "Float (single-precision)"))
  (returns (L01 :type "Vector Structure") (L02 :type "Vector Structure") (L03 :type "Vector Structure") (L04 :type "Vector Structure") (L05 :type "Vector Structure") (L06 :type "Vector Structure") (L07 :type "Vector Structure"))
  (bind _returnvalue (+ (* A B) A))
  (bind _returnvalue_2 (+ (* _returnvalue B) _returnvalue))
  (bind _returnvalue_3 (+ (* _returnvalue_2 B) _returnvalue_2))
  (bind _returnvalue_4 (+ (* _returnvalue_3 B) _returnvalue_3))
  (return A _returnvalue _returnvalue_2 _returnvalue_3 _returnvalue_4 (+ (* _returnvalue_4 B) _returnvalue_4) (0.0 0.0 0.0)))

(fn `UserConstructionScript`)