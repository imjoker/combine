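; Legacy Tier 2 square piece, apparently for a combine game: a cube with a box collider whose size and material follow its Level.
; Pure derives each level's size by compounding a base value by a growth factor, with L07 zeroed; the construction script applies it.
; ANIMATION lerps scale and extent to the next level on a timeline unless STOP, then increments Level.
; Tick reapplies the material; BeginPlay sets physics simulation and a random ID.
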(event `self.ReceiveTick`
  (params (DeltaSeconds :type "Float (single-precision)"))
  (`PrimitiveComponent.SetMaterial` (`self.SM_RCube`) 0 (select `/Game/Combine/Blueprint/Enum_Level` (`self.Level`) :`NewEnumerator0` "/Game/Combine/Mat/BasicAsset01.BasicAsset01" :`NewEnumerator1` "/Game/Combine/Mat/BasicAsset02.BasicAsset02" :`NewEnumerator2` "/Game/Combine/Mat/BasicAsset03.BasicAsset03" :`NewEnumerator3` "/Game/Combine/Mat/BasicAsset04.BasicAsset04" :`NewEnumerator4` "/Game/Combine/Mat/BasicAsset05.BasicAsset05" :`NewEnumerator5` "/Game/Combine/Mat/BasicAsset06.BasicAsset06" :!type "MaterialInterface Object Reference")))

(event `ANIMATION`
  (bind _level (`self.Level`))
  (bind (_l01 _l02 _l03 _l04 _l05 _l06) (`self.pure` (`self.basicscale`) (`self.basicscale1`)))
  (bind (_l01_2 _l02_2 _l03_2 _l04_2 _l05_2 _l06_2) (`self.pure` (`self.basicSCALE2`) (`self.basicscale1`)))
  (bind (_l01_3 _l02_3 _l03_3 _l04_3 _l05_3 _l06_3) (`self.pure` (`self.basicSCALE2`) (`self.basicscale1`)))
  (bind (_l01_4 _l02_4 _l03_4 _l04_4 _l05_4 _l06_4) (`self.pure` (`self.basicscale`) (`self.basicscale1`)))
  (bind _returnvalue (cast `/Game/Combine/Blueprint/Enum_Level` (`KismetMathLibrary.Conv_IntToByte` (+ (`KismetMathLibrary.Conv_ByteToInt` _level) 1))))
  ;[1 1 1] animation
  (set `self.CURRENT` (select `/Game/Combine/Blueprint/Enum_Level` _level :`NewEnumerator0` _l01 :`NewEnumerator1` _l02 :`NewEnumerator2` _l03 :`NewEnumerator3` _l04 :`NewEnumerator4` _l05 :`NewEnumerator5` _l06))
  (set `self.CURRENT2` (select `/Game/Combine/Blueprint/Enum_Level` _level :`NewEnumerator0` _l01_2 :`NewEnumerator1` _l02_2 :`NewEnumerator2` _l03_2 :`NewEnumerator3` _l04_2 :`NewEnumerator4` _l05_2 :`NewEnumerator5` _l06_2))
  (set `self.TARFETSCALE` (select `/Game/Combine/Blueprint/Enum_Level` _returnvalue :`NewEnumerator0` _l01_4 :`NewEnumerator1` _l02_4 :`NewEnumerator2` _l03_4 :`NewEnumerator3` _l04_4 :`NewEnumerator4` _l05_4 :`NewEnumerator5` _l06_4))
  (set `self.NewVar_0` (select `/Game/Combine/Blueprint/Enum_Level` _returnvalue :`NewEnumerator0` _l01_3 :`NewEnumerator1` _l02_3 :`NewEnumerator2` _l03_3 :`NewEnumerator3` _l04_3 :`NewEnumerator4` _l05_3 :`NewEnumerator5` _l06_3))
  (bind (_direction _lerp) (`Timeline|Timeline_0` :!via `PlayFromStart`)
    (:`Update`
      (if (not (`self.STOP`))
        (`SceneComponent.SetRelativeScale3D` (`self.SM_RCube`) (`KismetMathLibrary.VLerp` (`self.CURRENT`) (`self.TARFETSCALE`) _lerp))
        (`BoxComponent.SetBoxExtent` (`self.Box`) (`KismetMathLibrary.VLerp` (`self.CURRENT2`) (`self.NewVar_0`) _lerp) true)))
    (:`Finished`
      (set `self.Level` _returnvalue))))

(event `self.ReceiveBeginPlay`
  (`PrimitiveComponent.SetSimulatePhysics` (`self.Box`) (`self.Simulate`))
  (set `self.ID` (`KismetMathLibrary.RandomIntegerInRange` 0 999)))

(event `self.Box.OnComponentHit`
  (params (HitComponent :type "PrimitiveComponent Object Reference") (OtherActor :type "Actor Object Reference") (OtherComp :type "PrimitiveComponent Object Reference") (NormalImpulse :type "Vector Structure") (Hit :type "HitResult Structure (by ref)")))

(fn `pure`
  (params (A :type "Vector Structure") (B :type "Float (single-precision)"))
  (returns (L01 :type "Vector Structure") (L02 :type "Vector Structure") (L03 :type "Vector Structure") (L04 :type "Vector Structure") (L05 :type "Vector Structure") (L06 :type "Vector Structure") (L07 :type "Vector Structure"))
  (bind _returnvalue (+ (* A B) A))
  (bind _returnvalue_2 (+ (* _returnvalue B) _returnvalue))
  (bind _returnvalue_3 (+ (* _returnvalue_2 B) _returnvalue_2))
  (bind _returnvalue_4 (+ (* _returnvalue_3 B) _returnvalue_3))
  (return A _returnvalue _returnvalue_2 _returnvalue_3 _returnvalue_4 (+ (* _returnvalue_4 B) _returnvalue_4) (0.0 0.0 0.0)))

(fn `UserConstructionScript`
  (bind _level (`self.Level`))
  (bind (_l01 _l02 _l03 _l04 _l05 _l06) (`self.pure` (`self.basicSCALE2`) (`self.basicscale1`)))
  (bind (_l01_2 _l02_2 _l03_2 _l04_2 _l05_2 _l06_2) (`self.pure` (`self.basicscale`) (`self.basicscale1`)))
  (`SceneComponent.SetRelativeScale3D` (`self.SM_RCube`) (select `/Game/Combine/Blueprint/Enum_Level` _level :`NewEnumerator0` _l01_2 :`NewEnumerator1` _l02_2 :`NewEnumerator2` _l03_2 :`NewEnumerator3` _l04_2 :`NewEnumerator4` _l05_2 :`NewEnumerator5` _l06_2))
  (`BoxComponent.SetBoxExtent` (`self.Box`) (select `/Game/Combine/Blueprint/Enum_Level` _level :`NewEnumerator0` _l01 :`NewEnumerator1` _l02 :`NewEnumerator2` _l03 :`NewEnumerator3` _l04 :`NewEnumerator4` _l05 :`NewEnumerator5` _l06) true)
  (`PrimitiveComponent.SetMaterial` (`self.SM_RCube`) 0 (select `/Game/Combine/Blueprint/Enum_Level` _level :`NewEnumerator0` "/Game/Combine/Mat/BasicAsset01.BasicAsset01" :`NewEnumerator1` "/Game/Combine/Mat/BasicAsset02.BasicAsset02" :`NewEnumerator2` "/Game/Combine/Mat/BasicAsset03.BasicAsset03" :`NewEnumerator3` "/Game/Combine/Mat/BasicAsset04.BasicAsset04" :`NewEnumerator4` "/Game/Combine/Mat/BasicAsset05.BasicAsset05" :`NewEnumerator5` "/Game/Combine/Mat/BasicAsset06.BasicAsset06" :!type "MaterialInterface Object Reference")))