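; Actor component that supports combining two actors into a new one.
; Attach stores a goal and raises a combine flag, but Tick acts on nothing and the goal-based velocity-target logic is disconnected.
; Merge spawns the Output class midway between both owners with their scales summed, leaving removal of the owner to a separate Delete function.
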(event `self.ReceiveTick`
  (params (DeltaSeconds :type "Float (single-precision)"))
  (if (`self.TimeToCombine`)
    _))

(fn `Attach`
  (params (NewGoal :type "Actor Object Reference"))
  (set `self.Goal` NewGoal)
  (set `self.TimeToCombine` true))

(fn `Delete`
  (`Actor.K2_DestroyActor` (`self.GetOwner`)))

(fn `Merge`
  (params (Other :type "/Game/Blueprints/Combine Object Reference"))
  (bind _returnvalue (`self.GetOwner` Other))
  (bind _returnvalue_2 (`self.GetOwner`))
  (bind _returnvalue_3 (`Actor.K2_GetActorLocation` _returnvalue_2))
  (`|SpawnActorFromClass` (`self.Output`) (`KismetMathLibrary.MakeTransform` (+ _returnvalue_3 (/ (- (`Actor.K2_GetActorLocation` _returnvalue) _returnvalue_3) 2.0)) (struct) (+ (`Actor.GetActorScale3D` _returnvalue) (`Actor.GetActorScale3D` _returnvalue_2))) "Undefined" "OverrideRootScale" null null))